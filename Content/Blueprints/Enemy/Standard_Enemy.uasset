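; Standard enemy Blueprint that handles its death effect and removal, building on a parent class.
; Tick runs the parent logic, then calls AoE and DIEEEEE on every frame that IsAlive is false.
; AoE only activates the blood splat cone effect, with no damage logic.
; DIEEEEE hides the mesh, waits briefly, then deactivates the effect and destroys the actor.
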(event Custom|DIEEEEE
  (Rendering|SetVisibility (Variables|Character|GetMesh) false false)
  (Utilities|FlowControl|Delay 2.0)
  (Components|Activation|Deactivate (Variables|Default|GetP_Blood_Splat_Cone))
  (Actor|DestroyActor))

(event EventBeginPlay
  (|CallParentFunction))

(event Collision|EventActorBeginOverlap
  (params (OtherActor :type Actor%20Object%20Reference))
  (|CallParentFunction OtherActor) ; This node is disabled and will not be called.\nDrag off pins to build functionality.
)

(event EventTick
  (params (DeltaSeconds :type Float%20%28single-precision%29))
  (|CallParentFunction DeltaSeconds)
  (if (not (Variables|Default|GetIsAlive))
    (CallFunction|AoE)
    (CallFunction|DIEEEEE)))

(fn ConstructionScript
  (|CallParentFunction))

(fn AoE
  (Components|Activation|Activate (Variables|Default|GetP_Blood_Splat_Cone) false))