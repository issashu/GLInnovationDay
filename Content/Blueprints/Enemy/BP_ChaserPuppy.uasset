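; Chaser puppy enemy Blueprint that adds a temporary movement speed boost.
; The construction script stores the walk speed as DefaultSpeed, and BoostSpeed scales the current speed by one plus SpeedMultiplier, then sets IsBoosted.
; A named timer restores DefaultSpeed after BoostDuration but leaves IsBoosted set.
; Nothing here calls BoostSpeed or implements chasing, as the event graph otherwise only forwards to the parent.
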(event Custom|BoostTimer
  (Utilities|Time|SetTimerbyFunctionName 0 "returnDefaultSpeed" (Variables|Default|GetboostDuration)))

(event EventBeginPlay
  (|CallParentFunction))

(event Collision|EventActorBeginOverlap
  (params (OtherActor :type Actor%20Object%20Reference))
  (|CallParentFunction OtherActor) ; This node is disabled and will not be called.\nDrag off pins to build functionality.
)

(event EventTick
  (params (DeltaSeconds :type Float%20%28single-precision%29))
  (|CallParentFunction DeltaSeconds))

(fn ConstructionScript
  (|CallParentFunction)
  (Variables|Default|SetdefaultSpeed (Variables|/Script/Engine.CharacterMovementComponent|GetMaxWalkSpeed (Variables|Character|GetCharacterMovement))))

(fn BoostSpeed
  (Variables|/Script/Engine.CharacterMovementComponent|SetMaxWalkSpeed (Variables|Character|GetCharacterMovement) (* (+ (Variables|Default|GetspeedMultiplier) 1.0) (Variables|/Script/Engine.CharacterMovementComponent|GetMaxWalkSpeed (Variables|Character|GetCharacterMovement))))
  (Variables|Default|SetisBoosted true)
  (CallFunction|BoostTimer))

(fn ReturnDefaultSpeed
  (Variables|/Script/Engine.CharacterMovementComponent|SetMaxWalkSpeed (Variables|Character|GetCharacterMovement) (Variables|Default|GetdefaultSpeed)))