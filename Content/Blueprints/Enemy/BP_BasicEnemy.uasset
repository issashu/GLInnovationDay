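; BP_BasicEnemy is a basic enemy Blueprint that tracks health, damage and an alive flag, which starts true in the Construction Script.
; Every Tick it adds HealingPerTick to Health with no cap or alive check, then clears IsAlive if Health is zero or below.
; Takedamage subtracts from Health and GetDamage returns the enemy's Damage value; neither is called within this Blueprint.
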(event EventBeginPlay)

(event Collision|EventActorBeginOverlap
  (params (OtherActor :type Actor%20Object%20Reference)))

(event EventTick
  (params (DeltaSeconds :type Float%20%28single-precision%29))
  (CallFunction|HealDamage)
  (CallFunction|OnDeath))

(fn ConstructionScript
  (Variables|Default|SetIsAlive true))

(fn OnDeath
  (if (<= (Variables|Default|GetHealth) 0)
    (Variables|Default|SetIsAlive false)))

(fn Takedamage
  (params (damage :type Integer))
  (Variables|Default|SetHealth (- (Variables|Default|GetHealth) damage)))

(fn HealDamage
  (Variables|Default|SetHealth (+ (Variables|Default|GetHealth) (Variables|Default|GethealingPerTick))))

(fn GetDamage
  (return (Variables|Default|GetDamage)))