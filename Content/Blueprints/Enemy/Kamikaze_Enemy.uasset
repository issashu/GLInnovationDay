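; Kamikaze enemy Blueprint that sets off an area-effect particle burst when it dies, then removes itself.
; Tick polls IsAlive and, every frame it is false, calls AoE0 to activate the particle system and DIEEEEE to hide the mesh.
; After a short delay, DIEEEEE deactivates the particles and destroys the actor.
; The AoE is visual only here, with no damage logic.
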(event Custom|DIEEEEE
  (Rendering|SetVisibility (Variables|Character|GetMesh) false false)
  (Utilities|FlowControl|Delay 2.0)
  (Components|Activation|Deactivate (Variables|Default|GetParticleSystem))
  (Actor|DestroyActor))

(event EventBeginPlay
  (|CallParentFunction))

(event Collision|EventActorBeginOverlap
  (params (OtherActor :type Actor%20Object%20Reference))
  (|CallParentFunction OtherActor) ; This node is disabled and will not be called.\nDrag off pins to build functionality.
)

(event EventTick
  (params (DeltaSeconds :type Float%20%28single-precision%29))
  (|CallParentFunction DeltaSeconds)
  (if (not (Variables|Default|GetIsAlive))
    (CallFunction|AoE0)
    (CallFunction|DIEEEEE)))

(fn ConstructionScript
  (|CallParentFunction))

(fn AoE0
  (Components|Activation|Activate (Variables|Default|GetParticleSystem) false))